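; Save point actor that shows a prompt when the ganyu character is inside its box and provides a save menu.
; Box overlaps toggle the tip_g widget's text.
; The create_save_umg event, not called within this graph, adds Hp and Save_interface widgets and switches to UI-only input with a cursor.
; Leaving the box removes a valid save widget and restores game-only input, but leaves the Hp widget.
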(event OnComponentBeginOverlap(Box)
  (params (OverlappedComponent :type Primitive%20Component%20Object%20Reference) (OtherActor :type Actor%20Object%20Reference) (OtherComp :type Primitive%20Component%20Object%20Reference) (OtherBodyIndex :type Integer) (bFromSweep :type Boolean) (SweepResult :type Hit%20Result%20Structure%20%28by%20ref%29))
  (bind _asganyu (Utilities|Casting|CastToganyu OtherActor))
  (Variables|Default|Setbp_ganyu_object _asganyu)
  (bind _astip_g (Utilities|Casting|CastTotip_g (UserInterface|GetWidget (Variables|Default|Gettip_g))))
  (Variables|/Script/UMG.Widget|SetVisibility (Variables|/Game/bp/logic/widget/tip_g.tip_g_C|Getword_g _astip_g) "Visible"))

(event OnComponentEndOverlap(Box)
  (params (OverlappedComponent :type Primitive%20Component%20Object%20Reference) (OtherActor :type Actor%20Object%20Reference) (OtherComp :type Primitive%20Component%20Object%20Reference) (OtherBodyIndex :type Integer))
  (bind _returnvalue (Game|GetPlayerController 0))
  (bind _save_interface_widget (Variables|Default|Getsave_interface_widget))
  (Utilities|Casting|CastToganyu OtherActor)
  (bind _astip_g (Utilities|Casting|CastTotip_g (UserInterface|GetWidget (Variables|Default|Gettip_g))))
  (Variables|/Script/UMG.Widget|SetVisibility (Variables|/Game/bp/logic/widget/tip_g.tip_g_C|Getword_g _astip_g) "Hidden")
  (Utilities|IsValid _save_interface_widget
    (:Is%20Valid
      (Widget|RemovefromParent _save_interface_widget)
      (Variables|/Script/Engine.PlayerController|SetbShowMouseCursor _returnvalue false)
      (Input|SetInputModeGameOnly _returnvalue false))))

(event Custom|create_save_umg
  (bind _returnvalue (UserInterface|CreateWidget "/Game/bp/logic/widget/hp.hp_C"))
  (bind _returnvalue_2 (UserInterface|CreateWidget "/Game/bp/logic/widget/save_interface.save_interface_C"))
  (Default|Init _returnvalue_2 false false)
  (bind _output_get (Variables|Default|Setsave_interface_widget _returnvalue_2))
  (UserInterface|Viewport|AddtoViewport _returnvalue 0)
  (bind _output_get_2 (Variables|Default|Setplayer_controller (Game|GetPlayerController 0)))
  (Input|SetInputModeUIOnly _output_get_2 (Variables|Default|Getsave_interface_widget) "DoNotLock" false)
  (Variables|/Script/Engine.PlayerController|SetbShowMouseCursor (Variables|Default|Getplayer_controller) true))

(event EventBeginPlay
  (bind _astip_g (Utilities|Casting|CastTotip_g (UserInterface|GetWidget (Variables|Default|Gettip_g))))
  (Variables|/Script/UMG.Widget|SetVisibility (Variables|/Game/bp/logic/widget/tip_g.tip_g_C|Getword_g _astip_g) "Hidden"))

(event Collision|EventActorBeginOverlap
  (params (OtherActor :type Actor%20Object%20Reference)))

(event EventTick
  (params (DeltaSeconds :type Float%20%28single-precision%29)))

(fn ConstructionScript)